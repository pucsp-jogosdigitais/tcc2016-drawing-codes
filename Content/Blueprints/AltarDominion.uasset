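; AltarDominion is a domination altar that awards points to hero characters standing inside its cylinder.
; Cylinder overlap events set an inside flag for each of Magnus, Mayah, Erin and Melkor.
; A one-second loop from BeginPlay reads those flags and adds PontosPorSeg to each occupant's score through character references in TccGameState.
; Magnus and Mayah also gain a small UltBar charge each tick, while Erin and Melkor gain only points.
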(event `Verificacao`
  ;[1 1 1] Verificacao Tick
  (`|ExecutionSequence`
    (:`then_0`
      (if (`self.MagnusDentro`)
        (bind _ascharacter_magnus (cast `/Game/Blueprints/Personagens/Magnus/Character_Magnus` (`/Game/Blueprints/Framework/TccGameState.CharRef_Magnus` (stale `self.ReceiveBeginPlay` _astcc_game_state))))
        (set `/Game/Blueprints/Personagens/Magnus/Character_Magnus.Pontos` (+ (`/Game/Blueprints/Personagens/Magnus/Character_Magnus.Pontos` _ascharacter_magnus) (`self.PontosPorSeg`)) _ascharacter_magnus)
        (set `/Game/Blueprints/Personagens/Magnus/Character_Magnus.UltBar` (+ (`/Game/Blueprints/Personagens/Magnus/Character_Magnus.UltBar` _ascharacter_magnus) 0.01) _ascharacter_magnus)))
    (:`then_1`
      (if (`self.MayahDentro`)
        (bind _ascharacter_mayah (cast `/Game/Blueprints/Personagens/Mayah/Character_Mayah` (`/Game/Blueprints/Framework/TccGameState.CharRef_Mayah` (stale `self.ReceiveBeginPlay` _astcc_game_state))))
        (set `/Game/Blueprints/Personagens/Mayah/Character_Mayah.Pontos` (+ (`/Game/Blueprints/Personagens/Mayah/Character_Mayah.Pontos` _ascharacter_mayah) (`self.PontosPorSeg`)) _ascharacter_mayah)
        (set `/Game/Blueprints/Personagens/Mayah/Character_Mayah.UltBar` (+ (`/Game/Blueprints/Personagens/Mayah/Character_Mayah.UltBar` _ascharacter_mayah) 0.01) _ascharacter_mayah)))
    (:`then_2`
      (if (`self.ErinDentro`)
        (bind _ascharacter_erin (cast `/Game/Blueprints/Personagens/Erin/Character_Erin` (`/Game/Blueprints/Framework/TccGameState.CharRef_Erin` (stale `self.ReceiveBeginPlay` _astcc_game_state))))
        (set `/Game/Blueprints/Personagens/Erin/Character_Erin.Pontos` (+ (`/Game/Blueprints/Personagens/Erin/Character_Erin.Pontos` _ascharacter_erin) (`self.PontosPorSeg`)) _ascharacter_erin)))
    (:`then_3`
      (if (`self.MelkorDentro`)
        (bind _ascharacter_melkor (cast `/Game/Blueprints/Personagens/Melkor/Character_Melkor` (`/Game/Blueprints/Framework/TccGameState.CharRef_Melkor` (stale `self.ReceiveBeginPlay` _astcc_game_state))))
        (set `/Game/Blueprints/Personagens/Melkor/Character_Melkor.Pontos` (+ (`/Game/Blueprints/Personagens/Melkor/Character_Melkor.Pontos` _ascharacter_melkor) (`self.PontosPorSeg`)) _ascharacter_melkor)))))

(event `self.ReceiveBeginPlay`
  ;[1 1 1] Verificacao Tick
  (bind _astcc_game_state (cast `/Game/Blueprints/Framework/TccGameState` (`GameplayStatics.GetGameState`)))
  (`self.Verificacao` :!label _label)
  (`KismetSystemLibrary.Delay` 1.0)
  (goto _label))

(event `self.Cylinder.OnComponentBeginOverlap`
  (params (OverlappedComponent :type "PrimitiveComponent Object Reference") (OtherActor :type "Actor Object Reference") (OtherComp :type "PrimitiveComponent Object Reference") (OtherBodyIndex :type Integer) (bFromSweep :type Boolean) (SweepResult :type "HitResult Structure (by ref)"))
  ;[1 1 1] Entrou
  (`|ExecutionSequence`
    (:`then_0`
      (cast `/Game/Blueprints/Personagens/Magnus/Character_Magnus` OtherActor)
      (set `self.MagnusDentro` true))
    (:`then_1`
      (cast `/Game/Blueprints/Personagens/Mayah/Character_Mayah` OtherActor)
      (set `self.MayahDentro` true))
    (:`then_2`
      (cast `/Game/Blueprints/Personagens/Erin/Character_Erin` OtherActor)
      (set `self.ErinDentro` true))
    (:`then_3`
      (cast `/Game/Blueprints/Personagens/Melkor/Character_Melkor` OtherActor)
      (set `self.MelkorDentro` true))))

(event `self.Cylinder.OnComponentEndOverlap`
  (params (OverlappedComponent :type "PrimitiveComponent Object Reference") (OtherActor :type "Actor Object Reference") (OtherComp :type "PrimitiveComponent Object Reference") (OtherBodyIndex :type Integer))
  ;[1 1 1] Saiu
  (`|ExecutionSequence`
    (:`then_0`
      (cast `/Game/Blueprints/Personagens/Magnus/Character_Magnus` OtherActor)
      (set `self.MagnusDentro` false))
    (:`then_1`
      (cast `/Game/Blueprints/Personagens/Mayah/Character_Mayah` OtherActor)
      (set `self.MayahDentro` false))
    (:`then_2`
      (cast `/Game/Blueprints/Personagens/Erin/Character_Erin` OtherActor)
      (set `self.ErinDentro` false))
    (:`then_3`
      (cast `/Game/Blueprints/Personagens/Melkor/Character_Melkor` OtherActor)
      (set `self.MelkorDentro` false))))

(fn `UserConstructionScript`)