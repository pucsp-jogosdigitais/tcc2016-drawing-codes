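; Shared local-multiplayer camera actor that frames two to four players, becoming the view target of their controllers on BeginPlay.
; BeginPlay reads the player count from TccGameInstance and caches the player characters.
; Each Tick finds the farthest-apart pair (or the only pair), then eases the actor with VInterpTo toward their summed location over Divisor.
; Spring arm length scales with that pair's distance, using a shorter ratio for two players, and the distance prints for debugging.
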(event `self.ReceiveBeginPlay`
  (`PlayerController.SetViewTargetWithBlend` (`GameplayStatics.GetPlayerController` 2) self 0.0 "VTBlend_Linear" 0.0 false)
  (`PlayerController.SetViewTargetWithBlend` (`GameplayStatics.GetPlayerController` 3) self 0.0 "VTBlend_Linear" 0.0 false)
  (`PlayerController.SetViewTargetWithBlend` (`GameplayStatics.GetPlayerController` 1) self 0.0 "VTBlend_Linear" 0.0 false)
  (`PlayerController.SetViewTargetWithBlend` (`GameplayStatics.GetPlayerController` 0) self 0.0 "VTBlend_Linear" 0.0 false)
  (bind _astcc_game_instance (cast `/Game/Blueprints/Framework/TccGameInstance` (`GameplayStatics.GetGameInstance`)))
  (switch `int` (`/Game/Blueprints/Framework/TccGameInstance.NmrPlayers` _astcc_game_instance)
    (:`2`
      (`KismetArrayLibrary.Array_Add` (`self.Players`) (`GameplayStatics.GetPlayerCharacter` 0))
      (`KismetArrayLibrary.Array_Add` (`self.Players`) (`GameplayStatics.GetPlayerCharacter` 1))
      (`self.ArrayToCvariables`)
      (set `self.NmrPlayers` "2"))
    (:`3`
      (`KismetArrayLibrary.Array_Add` (`self.Players`) (`GameplayStatics.GetPlayerCharacter` 0))
      (`KismetArrayLibrary.Array_Add` (`self.Players`) (`GameplayStatics.GetPlayerCharacter` 1))
      (`KismetArrayLibrary.Array_Add` (`self.Players`) (`GameplayStatics.GetPlayerCharacter` 2))
      (`self.ArrayToCvariables`)
      (set `self.NmrPlayers` "3"))
    (:`4`
      (`KismetArrayLibrary.Array_Add` (`self.Players`) (`GameplayStatics.GetPlayerCharacter` 0))
      (`KismetArrayLibrary.Array_Add` (`self.Players`) (`GameplayStatics.GetPlayerCharacter` 1))
      (`KismetArrayLibrary.Array_Add` (`self.Players`) (`GameplayStatics.GetPlayerCharacter` 2))
      (`KismetArrayLibrary.Array_Add` (`self.Players`) (`GameplayStatics.GetPlayerCharacter` 3))
      (`self.ArrayToCvariables`)
      (set `self.NmrPlayers` "4"))))

(event `self.ReceiveTick`
  (params (DeltaSeconds :type "Float (single-precision)"))
  (switch `string` (`self.NmrPlayers`)
    (:`2`
      (`self.2 Players`))
    (:`3`
      (`self. 3 Players`))
    (:`4`
      (`self.4 Players`))))

(event `4 Players`
  (bind _index (`self.Index`))
  (bind (_indexofmaxvalue _maxvalue) (`KismetMathLibrary.MaxOfFloatArray` (`|MakeArray` (`KismetMathLibrary.Abs` (`KismetMathLibrary.VSize` (- (`self.K2_GetActorLocation` (`self.c1`)) (`self.K2_GetActorLocation` (`self.c2`))))) (`KismetMathLibrary.Abs` (`KismetMathLibrary.VSize` (- (`self.K2_GetActorLocation` (`self.c1`)) (`self.K2_GetActorLocation` (`self.c3`))))) (`KismetMathLibrary.Abs` (`KismetMathLibrary.VSize` (- (`self.K2_GetActorLocation` (`self.c1`)) (`self.K2_GetActorLocation` (`self.c4`))))) (`KismetMathLibrary.Abs` (`KismetMathLibrary.VSize` (- (`self.K2_GetActorLocation` (`self.c2`)) (`self.K2_GetActorLocation` (`self.c3`))))) (`KismetMathLibrary.Abs` (`KismetMathLibrary.VSize` (- (`self.K2_GetActorLocation` (`self.c2`)) (`self.K2_GetActorLocation` (`self.c4`))))) (`KismetMathLibrary.Abs` (`KismetMathLibrary.VSize` (- (`self.K2_GetActorLocation` (`self.c3`)) (`self.K2_GetActorLocation` (`self.c4`))))))))
  ;[1 1 1] 4 Players
  (set `self.Index` _indexofmaxvalue)
  (set `self.Distance` (`KismetMathLibrary.Conv_DoubleToVector` _maxvalue))
  (if (== _index 0)
    (`self.Func 1-2`)
    (bind _output_get (set `self.Focus` (`KismetMathLibrary.VInterpTo` (`self.OldPosition`) (`self.NewPosition`) (`GameplayStatics.GetWorldDeltaSeconds`) (`self.InterpSpeed`)) :!label _label))
    (`self.K2_SetActorLocation` _output_get)
    (set `self.OldPosition` (`self.K2_GetActorLocation`))
    (set `SpringArmComponent.TargetArmLength` (/ (`self.VectorLengh`) 2.0) (`self.SpringArm`))
    ;[1 1 1] 3 Players
    (`KismetSystemLibrary.PrintString` (`KismetStringLibrary.Conv_DoubleToString` (`self.VectorLengh`)) true false (struct :`G` 0.66 :`B` 1.0 :`A` 1.0) 0.0)
    (elif (== _index 1)
      (`self.Func 1-3`)
      (goto _label)
      (elif (== _index 2)
        (`self.Func 1-4`)
        (goto _label)
        (elif (== _index 3)
          (`self.Func 2-3`)
          (goto _label)
          (elif (== _index 4)
            (`self.Func 2-4`)
            (goto _label)
            (elif (== _index 5)
              (`self.Func 3-4`)
              (goto _label))))))))

(event `3 Players`
  (bind _index (`self.Index`))
  (bind (_indexofmaxvalue _maxvalue) (`KismetMathLibrary.MaxOfFloatArray` (`|MakeArray` (`KismetMathLibrary.Abs` (`KismetMathLibrary.VSize` (- (`self.K2_GetActorLocation` (`self.c1`)) (`self.K2_GetActorLocation` (`self.c2`))))) (`KismetMathLibrary.Abs` (`KismetMathLibrary.VSize` (- (`self.K2_GetActorLocation` (`self.c1`)) (`self.K2_GetActorLocation` (`self.c3`))))) (`KismetMathLibrary.Abs` (`KismetMathLibrary.VSize` (- (`self.K2_GetActorLocation` (`self.c2`)) (`self.K2_GetActorLocation` (`self.c3`))))))))
  ;[1 1 1] 3 Players
  (set `self.Index` _indexofmaxvalue)
  (set `self.Distance` (`KismetMathLibrary.Conv_DoubleToVector` _maxvalue))
  (if (== _index 0)
    (`self.Func 1-2`)
    (bind _output_get (set `self.Focus` (`KismetMathLibrary.VInterpTo` (`self.OldPosition`) (`self.NewPosition`) (`GameplayStatics.GetWorldDeltaSeconds`) (`self.InterpSpeed`)) :!label _label_2))
    (`self.K2_SetActorLocation` _output_get)
    (set `self.OldPosition` (`self.K2_GetActorLocation`))
    (set `SpringArmComponent.TargetArmLength` (/ (`self.VectorLengh`) 2.0) (`self.SpringArm`))
    (`KismetSystemLibrary.PrintString` (`KismetStringLibrary.Conv_DoubleToString` (`self.VectorLengh`)) true false (struct :`G` 0.66 :`B` 1.0 :`A` 1.0) 0.0)
    (elif (== _index 1)
      (`self.Func 1-3`)
      (goto _label_2)
      (elif (== _index 2)
        (`self.Func 2-3`)
        (goto _label_2)))))

(event `2 Players`
  (bind _returnvalue (`self.K2_GetActorLocation` (`self.c1`)))
  (bind _returnvalue_2 (`self.K2_GetActorLocation` (`self.c2`)))
  ;[1 1 1] 2 Players
  (`|ExecutionSequence`
    (:`then_0`
      (set `self.NewPosition` (/ (+ _returnvalue _returnvalue_2) (`self.Divisor`)))
      (bind _output_get (set `self.Focus` (`KismetMathLibrary.VInterpTo` (`self.OldPosition`) (`self.NewPosition`) (`GameplayStatics.GetWorldDeltaSeconds`) (`self.InterpSpeed`))))
      (set `self.VectorLengh` (`KismetMathLibrary.VSize` (- _returnvalue _returnvalue_2)))
      (`self.K2_SetActorLocation` _output_get)
      (set `self.OldPosition` (`self.K2_GetActorLocation`))
      (set `SpringArmComponent.TargetArmLength` (/ (`self.VectorLengh`) 4.0) (`self.SpringArm`))
      (`KismetSystemLibrary.PrintString` (`KismetStringLibrary.Conv_DoubleToString` (`self.VectorLengh`)) true false (struct :`G` 0.66 :`B` 1.0 :`A` 1.0) 0.0))))

(fn `ArrayToCvariables`
  (set `self.c1` (`KismetArrayLibrary.Array_Get` (`self.Players`)))
  (set `self.c2` (`KismetArrayLibrary.Array_Get` (`self.Players`) 1))
  (set `self.c3` (`KismetArrayLibrary.Array_Get` (`self.Players`) 2))
  (set `self.c4` (`KismetArrayLibrary.Array_Get` (`self.Players`) 3)))

(fn `Func 1-2`
  (bind _returnvalue (`self.K2_GetActorLocation` (`self.c2`)))
  (bind _returnvalue_2 (`self.K2_GetActorLocation` (`self.c1`)))
  (set `self.NewPosition` (/ (+ _returnvalue_2 _returnvalue) (`self.Divisor`)))
  (set `self.VectorLengh` (`KismetMathLibrary.VSize` (- _returnvalue_2 _returnvalue))))

(fn `Func 1-3`
  (bind _returnvalue (`self.K2_GetActorLocation` (`self.c3`)))
  (bind _returnvalue_2 (`self.K2_GetActorLocation` (`self.c1`)))
  (set `self.NewPosition` (/ (+ _returnvalue_2 _returnvalue) (`self.Divisor`)))
  (set `self.VectorLengh` (`KismetMathLibrary.VSize` (- _returnvalue_2 _returnvalue))))

(fn `Func 1-4`
  (bind _returnvalue (`self.K2_GetActorLocation` (`self.c4`)))
  (bind _returnvalue_2 (`self.K2_GetActorLocation` (`self.c1`)))
  (set `self.NewPosition` (/ (+ _returnvalue_2 _returnvalue) (`self.Divisor`)))
  (set `self.VectorLengh` (`KismetMathLibrary.VSize` (- _returnvalue_2 _returnvalue))))

(fn `Func 2-3`
  (bind _returnvalue (`self.K2_GetActorLocation` (`self.c3`)))
  (bind _returnvalue_2 (`self.K2_GetActorLocation` (`self.c2`)))
  (set `self.NewPosition` (/ (+ _returnvalue_2 _returnvalue) (`self.Divisor`)))
  (set `self.VectorLengh` (`KismetMathLibrary.VSize` (- _returnvalue_2 _returnvalue))))

(fn `Func 2-4`
  (bind _returnvalue (`self.K2_GetActorLocation` (`self.c4`)))
  (bind _returnvalue_2 (`self.K2_GetActorLocation` (`self.c2`)))
  (set `self.NewPosition` (/ (+ _returnvalue_2 _returnvalue) (`self.Divisor`)))
  (set `self.VectorLengh` (`KismetMathLibrary.VSize` (- _returnvalue_2 _returnvalue))))

(fn `Func 3-4`
  (bind _returnvalue (`self.K2_GetActorLocation` (`self.c4`)))
  (bind _returnvalue_2 (`self.K2_GetActorLocation` (`self.c3`)))
  (set `self.NewPosition` (/ (+ _returnvalue_2 _returnvalue) (`self.Divisor`)))
  (set `self.VectorLengh` (`KismetMathLibrary.VSize` (- _returnvalue_2 _returnvalue))))

(fn `UserConstructionScript`)