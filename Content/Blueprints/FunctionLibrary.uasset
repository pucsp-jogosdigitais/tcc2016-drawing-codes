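; Blueprint function library of player 1 helpers for positions and right analog stick (AnalogicoDireito) data.
; The getter casts player character 0 to Character_Magnus and returns its stored right-stick vector.
; The position function returns the controlled pawn's transform, lowered by a fixed Z offset with unit scale.
; Despite its name, the Set function writes nothing, returning that same transform shifted by the stick vector.
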(fn `pl1_Get_AnalogicoDireito`
  (returns (Position :type "Vector Structure"))
  (bind _ascharacter_magnus (cast `/Game/Blueprints/Personagens/Magnus/Character_Magnus` (`GameplayStatics.GetPlayerCharacter` null))
    (:`then`
      _)
    (:`CastFailed`
      _))
  (return (`/Game/Blueprints/Personagens/Magnus/Character_Magnus.AnalogicoDireitoVector` _ascharacter_magnus)))

(fn `pl1_Player_Position`
  (returns (Posicao :type "Transform Structure"))
  (bind _returnvalue (`Controller.K2_GetPawn` (`GameplayStatics.GetPlayerController` null)))
  (return (`KismetMathLibrary.MakeTransform` (`KismetMathLibrary.MakeVector` (.x (`Actor.K2_GetActorLocation` _returnvalue)) (.y (`Actor.K2_GetActorLocation` _returnvalue)) (- (.z (`Actor.K2_GetActorLocation` _returnvalue)) 80.0)) (`Actor.K2_GetActorRotation` _returnvalue))))

(fn `pl1_Set_AnalogicoDireito`
  (returns (Posicao :type "Transform Structure"))
  (bind _returnvalue (`Controller.K2_GetPawn` (`GameplayStatics.GetPlayerController` null)))
  (bind _ascharacter_magnus (cast `/Game/Blueprints/Personagens/Magnus/Character_Magnus` (`GameplayStatics.GetPlayerCharacter` null))
    (:`then`
      _)
    (:`CastFailed`
      _))
  (return (`KismetMathLibrary.MakeTransform` (+ (`/Game/Blueprints/Personagens/Magnus/Character_Magnus.AnalogicoDireitoVector` _ascharacter_magnus) (`KismetMathLibrary.MakeVector` (.x (`Actor.K2_GetActorLocation` _returnvalue)) (.y (`Actor.K2_GetActorLocation` _returnvalue)) (- (.z (`Actor.K2_GetActorLocation` _returnvalue)) 80.0))) (`Actor.K2_GetActorRotation` _returnvalue))))