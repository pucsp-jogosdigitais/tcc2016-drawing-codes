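; TccHUD is the match HUD that creates player widgets and runs the Domination mode's match timer.
; BeginPlay checks the GameInstance mode, adding the main widget for Domination, and Tick counts minutes and seconds down once the match has started.
; When time expires, a one-shot event shows an end countdown, waits, clears widgets, opens MagnusWinMap and adds the end-game widget.
; CreateMatchWidgets adds one distinct widget per player, up to four.
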(event `self.ReceiveBeginPlay`
  (bind _astcc_game_instance (cast `/Game/Blueprints/Framework/TccGameInstance` (`GameplayStatics.GetGameInstance`)))
  (switch `string` (`/Game/Blueprints/Framework/TccGameInstance.ModoDeJogo` _astcc_game_instance)
    (:`DominationGM`
      (set `self.Domination` true)
      (bind _returnvalue (`|CreateWidget` "/Game/Blueprints/Framework/TccWidgetBP.TccWidgetBP_C"))
      (`UserWidget.AddToViewport` _returnvalue 0))))

(event `self.ReceiveTick`
  (params (DeltaSeconds :type "Float (single-precision)"))
  ;[1 1 1] Cronometro
  (if (`self.Domination`)
    (if (`self.JogoComecou(Map)`)
      (`|ExecutionSequence`
        (:`then_0`
          (if (== (`self.segundos_60_Timer`) 0)
            (set `self.segundos_60` 59.0)
            (set `self.minutos` (- (`self.minutos`) 1))))
        (:`then_1`
          (bind _output_get (set `self.segundos_60` (- (`self.segundos_60`) DeltaSeconds)))
          (set `self.segundos_60_Timer` (`KismetMathLibrary.Round` _output_get)))
        (:`then_2`
          ;[1 1 1] Fim de partida
          (if (<= (`self.segundos_60_Timer`) 0)
            (if (< (`self.minutos`) 1)
              (`/Engine/EditorBlueprintResources/StandardMacros.DoOnce` false
                (:`Completed`
                  (`self.CustomEvent_0`))))))))))

(event `CustomEvent_0`
  ;[1 1 1] Fim de partida
  (bind _returnvalue (`|CreateWidget` "/Game/Mapas/Widgets/InGameHUD/ContagemFimPartida.ContagemFimPartida_C"))
  (`UserWidget.AddToViewport` _returnvalue 0)
  (`KismetSystemLibrary.Delay` 8.0)
  (`WidgetLayoutLibrary.RemoveAllWidgets`)
  (`GameplayStatics.OpenLevel` "MagnusWinMap")
  (bind _returnvalue_2 (`|CreateWidget` "/Game/Blueprints/Framework/EndGameWidget.EndGameWidget_C"))
  (`UserWidget.AddToViewport` _returnvalue_2 0))

(event `CreateMatchWidgets`
  ;[1 1 1] Players widgets
  (bind _astcc_game_instance (cast `/Game/Blueprints/Framework/TccGameInstance` (`GameplayStatics.GetGameInstance`)))
  (switch `int` (`/Game/Blueprints/Framework/TccGameInstance.NmrPlayers` _astcc_game_instance)
    (:`1`
      (bind _returnvalue (`|CreateWidget` "/Game/Mapas/Widgets/InGameHUD/1Player_Widget.1Player_Widget_C"))
      (`UserWidget.AddToViewport` _returnvalue 0))
    (:`2`
      (bind _returnvalue_2 (`|CreateWidget` "/Game/Mapas/Widgets/InGameHUD/1Player_Widget.1Player_Widget_C"))
      (`UserWidget.AddToViewport` _returnvalue_2 0)
      (bind _returnvalue_3 (`|CreateWidget` "/Game/Mapas/Widgets/InGameHUD/2Player_Widget.2Player_Widget_C"))
      (`UserWidget.AddToViewport` _returnvalue_3 0))
    (:`3`
      (bind _returnvalue_4 (`|CreateWidget` "/Game/Mapas/Widgets/InGameHUD/1Player_Widget.1Player_Widget_C"))
      (`UserWidget.AddToViewport` _returnvalue_4 0)
      (bind _returnvalue_5 (`|CreateWidget` "/Game/Mapas/Widgets/InGameHUD/2Player_Widget.2Player_Widget_C"))
      (`UserWidget.AddToViewport` _returnvalue_5 0)
      (bind _returnvalue_6 (`|CreateWidget` "/Game/Mapas/Widgets/InGameHUD/3Player_Widget.3Player_Widget_C"))
      (`UserWidget.AddToViewport` _returnvalue_6 0))
    (:`4`
      (bind _returnvalue_7 (`|CreateWidget` "/Game/Mapas/Widgets/InGameHUD/1Player_Widget.1Player_Widget_C"))
      (`UserWidget.AddToViewport` _returnvalue_7 0)
      (bind _returnvalue_8 (`|CreateWidget` "/Game/Mapas/Widgets/InGameHUD/2Player_Widget.2Player_Widget_C"))
      (`UserWidget.AddToViewport` _returnvalue_8 0)
      (bind _returnvalue_9 (`|CreateWidget` "/Game/Mapas/Widgets/InGameHUD/3Player_Widget.3Player_Widget_C"))
      (`UserWidget.AddToViewport` _returnvalue_9 0)
      (bind _returnvalue_10 (`|CreateWidget` "/Game/Mapas/Widgets/InGameHUD/4Player_Widget.4Player_Widget_C"))
      (`UserWidget.AddToViewport` _returnvalue_10 0))))

(fn `UserConstructionScript`)