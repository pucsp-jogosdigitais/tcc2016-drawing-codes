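; Collectible factory Blueprint, named for MelkorMap, that scatters a random handful of child actors, apparently power-ups, inside its Box volume.
; The construction script calls SpawnPowerUP, which adds one to three Child Actor components at random points in the box's scaled extent.
; Placement happens at construction, so it re-randomizes whenever the script reruns.
; A disconnected SpawnActor node for Coletavel_PowerUp remains unused.
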(fn `SpawnPowerUP`
  (bind _box (`self.Box`))
  (for _ (range (+ (`KismetMathLibrary.RandomIntegerInRange` 1 3) 1))
    (`AddComponent|Child Actor Component_2` :`RelativeTransform` (`KismetMathLibrary.Conv_VectorToTransform` (`KismetMathLibrary.RandomPointInBoundingBox` (`SceneComponent.RelativeLocation` _box) (`BoxComponent.GetScaledBoxExtent` _box))))))

(fn `UserConstructionScript`
  (`self.SpawnPowerUP`))